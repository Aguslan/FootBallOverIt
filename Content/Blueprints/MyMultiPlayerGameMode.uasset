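; Multiplayer game mode that assigns each player a spawn point according to how many players are present.
; Its ChoosePlayerStart override counts MyPlayerController actors and returns the MyPlayerStart whose PlayerStartTag equals that number as text, with no fallback when none matches.
; BeginPlay and Tick are empty, and the nodes that would create the W_InterfaceLvl widget and set game-and-UI input are disconnected.
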(event EventTick
  (params (DeltaSeconds :type Float%20%28single-precision%29)))

(event EventBeginPlay)

(fn ConstructionScript)

(fn ChoosePlayerStart
  (params (Player :type Controller%20Object%20Reference))
  (bind _outactors (Actor|GetAllActorsOfClass "/Game/Blueprints/MyPlayerController.MyPlayerController_C"))
  (bind _outactors_2 (Actor|GetAllActorsOfClass "/Game/Blueprints/MyPlayerStart.MyPlayerStart_C"))
  (for _array_element _outactors_2
    (if (== (Variables|/Script/Engine.PlayerStart|GetPlayerStartTag _array_element) (Utilities|String|ToString(Integer) (Utilities|Array|Length _outactors)))
      (return _array_element))))