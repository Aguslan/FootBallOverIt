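; Game instance Blueprint that manages multiplayer sessions for hosting, joining and leaving games.
; SessionHost creates a session with the given connection count and LAN flag, then opens Level1 as a listen server on success.
; SessionJoin joins a passed search result and DestoySession ends the session, both using the first player controller.
; Host and join results are only reported through printed text, with no further error handling.
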(event Custom|Session%20Host
  (params (PublicConnections :type Integer) (bUseLAN :type Boolean))
  (|Session (Game|GetPlayerController 0) PublicConnections bUseLAN
    (:OnSuccess
      (Development|PrintText "Session Success")
      (Game|OpenLevel(byObjectReference) "/Game/Maps/Level1.Level1" true "listen"))
    (:OnFailure
      (Development|PrintText "Error to create session"))))

(event Custom|Session%20Join
  (params (SearchResult :type Blueprint%20Session%20Result%20Structure%20%28by%20ref%29))
  (|JoinSession (Game|GetPlayerController 0) SearchResult
    (:OnSuccess
      (Development|PrintText "Join Session Success"))
    (:OnFailure
      (Development|PrintText "Error to Join session"))))

(event Custom|Destoy%20Session
  (|DestroySession (Game|GetPlayerController 0)))