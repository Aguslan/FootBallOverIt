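; BP_ItemUDBall is a ball item that cycles through random shot values from -2 to 2.
; BeginPlay picks a starting index, which sets the sphere's color material and the TxtShoots label.
; A Delay on Tick re-rolls the index every 1.7 seconds through the same display switch.
; The ReadyForChange comparison loop never runs because the flag starts false, and no overlap or pickup logic exists here.
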(event EventBeginPlay
  (Variables|Default|SetNumberSelected (Math|Random|RandomInteger 5))
  (Variables|Default|SetReadyForChange false)
  (switch int (Variables|Default|GetNumberSelected)
    (:0
      (Rendering|Material|SetMaterial (Variables|Default|GetSphere) 0 "/Game/Character/M_BallBlack.M_BallBlack")
      (Variables|Default|SetShotText "-2"))
    (:1
      (Rendering|Material|SetMaterial (Variables|Default|GetSphere) 0 "/Game/Material/M_Red.M_Red")
      (Variables|Default|SetShotText "-1"))
    (:2
      (Rendering|Material|SetMaterial (Variables|Default|GetSphere) 0 "/Game/Material/M_Yellow.M_Yellow")
      (Variables|Default|SetShotText "0"))
    (:3
      (Rendering|Material|SetMaterial (Variables|Default|GetSphere) 0 "/Game/Material/M_Green.M_Green")
      (Variables|Default|SetShotText "1"))
    (:4
      (Rendering|Material|SetMaterial (Variables|Default|GetSphere) 0 "/Game/Material/M_LightGreen.M_LightGreen")
      (Variables|Default|SetShotText "2")))
  (Rendering|Components|TextRender|SetText (Variables|Default|GettxtShoots) (Variables|Default|GetShotText)))

(event Collision|EventActorBeginOverlap
  (params (OtherActor :type Actor%20Object%20Reference)))

(event EventTick
  (params (DeltaSeconds :type Float%20%28single-precision%29))
  (bind _returnvalue (Math|Random|RandomInteger 5))
  (bind _returnvalue_2 (Math|Random|RandomInteger 5))
  (bind _returnvalue_3 (Math|Random|RandomIntegerinRange _returnvalue_2 _returnvalue))
  (Utilities|FlowControl|Delay 1.7)
  (while (Variables|Default|GetReadyForChange)
    (Math|Integer|CompareInt (Variables|Default|GetNumberSelected) _returnvalue_3
      (:>
        (Variables|Default|SetReadyForChange true :!label _label))
      (:==
        (Variables|Default|SetReadyForChange false))
      (:<
        (goto _label))))
  (Variables|Default|SetReadyForChange false)
  (Variables|Default|SetNumberSelected _returnvalue_3)
  (switch int (Variables|Default|GetNumberSelected)
    (:0
      (Rendering|Material|SetMaterial (Variables|Default|GetSphere) 0 "/Game/Character/M_BallBlack.M_BallBlack")
      (Variables|Default|SetShotText "-2"))
    (:1
      (Rendering|Material|SetMaterial (Variables|Default|GetSphere) 0 "/Game/Material/M_Red.M_Red")
      (Variables|Default|SetShotText "-1"))
    (:2
      (Rendering|Material|SetMaterial (Variables|Default|GetSphere) 0 "/Game/Material/M_Yellow.M_Yellow")
      (Variables|Default|SetShotText "0"))
    (:3
      (Rendering|Material|SetMaterial (Variables|Default|GetSphere) 0 "/Game/Material/M_Green.M_Green")
      (Variables|Default|SetShotText "1"))
    (:4
      (Rendering|Material|SetMaterial (Variables|Default|GetSphere) 0 "/Game/Material/M_LightGreen.M_LightGreen")
      (Variables|Default|SetShotText "2")))
  (Rendering|Components|TextRender|SetText (Variables|Default|GettxtShoots) (Variables|Default|GetShotText)))

(fn ConstructionScript)