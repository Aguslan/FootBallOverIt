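; BP_Ball_2 is a multiplayer physics ball that players launch by click-dragging on it, with limited shots.
; Drag direction becomes a stepped Y/Z impulse, sent via Server and Multicast events into RepNotify variables, as are material, name and trail state.
; Exhausted shots turn the ball black until it slows, then refill.
; Tick also drives the speed-based trail, name tag and crowd sounds, while BP_ItemUDBall pickups adjust shots and respawn.
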(event OnBeginCursorOver(Sphere)
  (params (TouchedComponent :type Primitive%20Component%20Object%20Reference))
  ;[1 1 1] Is On the Ball?
  (Variables|Default|SetIsOver true))

(event OnEndCursorOver(Sphere)
  (params (TouchedComponent :type Primitive%20Component%20Object%20Reference))
  ;[1 1 1] Is On the Ball?
  (Variables|Default|SetIsOver false))

(event OnComponentBeginOverlap(Sphere1)
  (params (OverlappedComponent :type Primitive%20Component%20Object%20Reference) (OtherActor :type Actor%20Object%20Reference) (OtherComp :type Primitive%20Component%20Object%20Reference) (OtherBodyIndex :type Integer) (bFromSweep :type Boolean) (SweepResult :type Hit%20Result%20Structure%20%28by%20ref%29))
  ;[1 1 1] Sound
  (if (Variables|Default|GetFirstSoundFall)
    (Audio|PlaySound2D "/Game/Sound/Fall.Fall" 1.0 1.0 0.0 0 0)
    (else
      (Variables|Default|SetFirstSoundFall true))))

(event Custom|Ready%20for%20Shot%20Multicast
  (params (Result%20X :type Float%20%28double-precision%29) (Result%20Y :type Float%20%28double-precision%29))
  ;[1 1 1] Logic For Impulse
  (Variables|CalculateShot|SetImpulse (Math|Vector|MakeVector 0.0 Result%20X Result%20Y)))

(event Custom|Ready%20for%20Shot%20Server
  (params (Result%20X :type Float%20%28double-precision%29) (Result%20Y :type Float%20%28double-precision%29))
  ;[1 1 1] Logic For Impulse
  (CallFunction|ReadyforShotMulticast Result%20X Result%20Y))

(event Custom|ChangeCurrentMaterialServer
  (params (InitialMaterial :type Material%20Object%20Reference))
  (CallFunction|ChangeCurrentMaterialMulticast InitialMaterial))

(event Custom|Change%20Color%20GREEN%20server
  (params (Material :type Material%20Interface%20Object%20Reference))
  (CallFunction|ChangeColorGREENMulticast Material))

(event Custom|Change%20Color%20GREEN%20multicast
  (params (Material :type Material%20Interface%20Object%20Reference))
  (Variables|Default|SetMaterial Material))

(event Custom|Ready%20for%20Trail%20Multicast
  (params (IsParticleAlim :type Boolean))
  ;[1 1 1] AnimParticles
  (Variables|Default|SetIsParticleAnim (not IsParticleAlim)))

(event Custom|Ready%20For%20Trail%20Server
  (params (IsParticleAnim :type Boolean))
  ;[1 1 1] AnimParticles
  (CallFunction|ReadyforTrailMulticast IsParticleAnim))

(event Custom|ChangeCurrentMaterialMulticast
  (params (InitialMaterial :type Material%20Object%20Reference))
  (Variables|Materials|SetCurrentMaterial InitialMaterial))

(event Custom|PlayerNameMulticast
  (params (Name :type Text))
  (Variables|Default|SetPlayerName Name))

(event Custom|PlayerNameServer
  (params (Name :type Text))
  (CallFunction|PlayerNameMulticast Name))

(event EventBeginPlay
  (CallFunction|PlayerNameServer (Utilities|Text|ToText(String) (Utilities|String|Append "Player " (Utilities|String|ToString(Integer) (Math|Random|RandomInteger 10)))))
  (CallFunction|ChangeCurrentMaterialServer (Variables|Materials|GetInitialMaterial))
  (Effects|Particles|Trails|EndTrails (Variables|Default|GetTrail))
  (Variables|Default|SetCountShot (Variables|Default|GetTiros)))

(event EventTick
  (params (DeltaSeconds :type Float%20%28single-precision%29))
  (bind _isparticleanim (Variables|Default|GetIsParticleAnim))
  (bind _sphere (Variables|Default|GetSphere))
  (bind _sphere_2 (Variables|Default|GetSphere))
  (bind _sphere_3 (Variables|Default|GetSphere))
  (bind _returnvalue (Transformation|GetComponentVelocity _sphere))
  (bind _returnvalue_2 (Transformation|GetComponentVelocity _sphere_3))
  (bind _returnvalue_3 (Transformation|GetWorldLocation _sphere_2))
  (Utilities|FlowControl|Sequence
    (:then_0
      ;[1 1 1] AnimParticles
      (Math|Float|CompareFloat (+ (Math|Float|Absolute(Float) (.y _returnvalue_2)) (Math|Float|Absolute(Float) (.z _returnvalue_2))) 5e+01
        (:>
          (if (not _isparticleanim)
            (CallFunction|ReadyforTrailServer (Variables|Default|GetIsParticleAnim))))
        (:<
          (if _isparticleanim
            (CallFunction|ReadyforTrailServer (Variables|Default|GetIsParticleAnim))))))
    (:then_1
      ;[1 1 1] Put CurrentMaterial if Material is Black
      (if (== (Rendering|Material|GetMaterial (Variables|Default|GetSphere) 0) (Variables|Materials|GetBlackMaterial))
        (Math|Integer|CompareInt (Variables|Default|GetCountShot) (Variables|Default|GetTiros)
          (:<
            (Math|Float|CompareFloat (+ (Math|Float|Absolute(Float) (.y _returnvalue)) (Math|Float|Absolute(Float) (.z _returnvalue))) 1e+01
              (:<
                (CallFunction|ChangeCurrentMaterialServer (Variables|Materials|GetInitialMaterial))
                (Variables|Default|SetCountShot (Variables|Default|GetTiros))))))))
    (:then_2
      (Transformation|SetWorldLocation (Variables|Default|GettxtPlayer) (Math|Vector|MakeVector (+ (.x _returnvalue_3) 0.0) (+ (.y _returnvalue_3) -1.2e+02) (+ (.z _returnvalue_3) 7e+01)) false false))
    (:then_3
      ;[1 1 1] Sound INchada
      (Utilities|FlowControl|Delay 15.0)
      (switch int (Variables|Default|GetIntSoundIncha)
        (:0
          (Variables|Default|SetIntSoundIncha 1)
          (Audio|PlaySound2D "/Game/Sound/InchadaAlong_Cue.InchadaAlong_Cue" 1.0 1.0 0.0 0 0))
        (:1
          (Variables|Default|SetIntSoundIncha 0)
          (Audio|PlaySound2D "/Game/Sound/InchadaBomb_Cue.InchadaBomb_Cue" 1.0 1.0 0.0 0 0))))))

(event Collision|EventActorBeginOverlap
  (params (OtherActor :type Actor%20Object%20Reference))
  ;[1 1 1] Bonus
  (if (Utilities|String|Contains (Utilities|GetObjectName OtherActor) "BP_ItemUDBall" true)
    (bind _asbp_item_udball (Utilities|Casting|CastToBP_ItemUDBall OtherActor))
    (Development|PrintString "Hello")
    (Math|Integer|CompareInt (+ (Variables|Default|GetCountShot) (Math|Conversions|ToInteger(Byte) (Utilities|String|ToString(Text) (Variables|/Game/Character/BP_ItemUDBall.BP_ItemUDBall_C|GetShotText _asbp_item_udball))))
      (:>
        (Variables|Default|SetCountShot (+ (Variables|Default|GetCountShot) (Math|Conversions|ToInteger(Byte) (Utilities|String|ToString(Text) (Variables|/Game/Character/BP_ItemUDBall.BP_ItemUDBall_C|GetShotText _asbp_item_udball))))))
      (:==
        (Variables|Default|SetCountShot 0 :!label _label))
      (:<
        (goto _label)))
    (Variables|Default|SetSpawn%20Transform (Math|Transform|MakeTransform (.location (Transformation|GetActorTransform _asbp_item_udball)) (.rotation (Transformation|GetActorTransform _asbp_item_udball)) (.scale (Transformation|GetActorTransform _asbp_item_udball))))
    (Development|PrintString (Utilities|GetDisplayName _asbp_item_udball))
    (Actor|DestroyActor _asbp_item_udball)
    (bind _asmy_multi_player_game_mode (Utilities|Casting|CastToMyMultiPlayerGameMode (Game|GetGameMode)))
    (Default|PuntosDisparo (Variables|/Game/Blueprints/MyMultiPlayerGameMode.MyMultiPlayerGameMode_C|GetInterLevel _asmy_multi_player_game_mode))
    (Utilities|FlowControl|Delay 1.0)
    (Game|SpawnActorfromClass "/Game/Character/BP_ItemUDBall.BP_ItemUDBall_C" (Variables|Default|GetSpawn%20Transform) "Undefined" 0 0)))

(event Input|ActionEvents|InputActionPressF
  (params (Key :type Key%20Structure :default "None"))
  (:Pressed
    (CallFunction|ChangeColorGREENServer "/Game/Material/M_Green.M_Green"))
  (:Released
    (CallFunction|ChangeColorGREENServer "/Game/Material/M_Red.M_Red")))

(event Input|MouseEvents|LeftMouseButton
  (params (Key :type Key%20Structure :default "None"))
  (:Pressed
    (if (Variables|Default|GetIsOver)
      (Variables|Default|SetReadyForShot true)
      (bind _returnvalue (Class|WidgetLayoutLibrary|GetMousePositiononViewport))
      (Variables|CalculateShot|SetPosIni _returnvalue)))
  (:Released
    (if (Variables|Default|GetReadyForShot)
      ;[1 1 1] is Fail Shot
      (bind _returnvalue_2 (Class|WidgetLayoutLibrary|GetMousePositiononViewport))
      (Math|Float|CompareFloat (.x _returnvalue_2) (.x (Variables|CalculateShot|GetPosIni))
        (:>
          _)
        (:<
          _))
      (Math|Integer|CompareInt (Variables|Default|GetCountShot)
        (:>
          (Audio|PlaySound2D "/Game/Sound/Shot_Ball.Shot_Ball" 1.0 1.0 0.0 0 0)
          (bind _returnvalue_3 (Class|WidgetLayoutLibrary|GetMousePositiononViewport))
          (bind _output_get (Variables|Default|SetResult (- (Variables|CalculateShot|GetPosIni) _returnvalue_3)))
          ;[1 1 1] Logic For Impulse
          (Math|Float|CompareFloat (.x _output_get) 0.0
            (:>
              (Math|Float|CompareFloat (.x _output_get) 75.0
                (:>
                  (Variables|CalculateShot|SetAuxX 125.0))
                (:==
                  (Variables|CalculateShot|SetAuxX 75.0))
                (:<
                  (Variables|CalculateShot|SetAuxX 3e+01))))
            (:==
              (Variables|CalculateShot|SetAuxX 0.0))
            (:<
              (Math|Float|CompareFloat (.x _output_get) -75.0
                (:>
                  (Variables|CalculateShot|SetAuxX -3e+01))
                (:==
                  (Variables|CalculateShot|SetAuxX -75.0))
                (:<
                  (Variables|CalculateShot|SetAuxX -125.0)))))
          (Math|Float|CompareFloat (.y _output_get) 0.0
            (:>
              (Math|Float|CompareFloat (.y _output_get) 75.0
                (:>
                  (Variables|CalculateShot|SetAuxY -125.0))
                (:==
                  (Variables|CalculateShot|SetAuxY -75.0))
                (:<
                  (Variables|CalculateShot|SetAuxY -3e+01)))
              (CallFunction|ReadyforShotServer (* (Variables|CalculateShot|GetAuxX) 7.0) (* (Variables|CalculateShot|GetAuxY) 8.0) :!label _label)
              (Variables|Default|SetReadyForShot false)
              (Variables|Default|SetCountShot (- (Variables|Default|GetCountShot) 1))
              ;[1 1 1] Material For Play
              (Math|Integer|CompareInt (Variables|Default|GetCountShot)
                (:==
                  (CallFunction|ChangeCurrentMaterialServer (Variables|Materials|GetBlackMaterial)))))
            (:==
              (Variables|CalculateShot|SetAuxY 0.0))
            (:<
              (Math|Float|CompareFloat (.y _output_get) -75.0
                (:>
                  (Variables|CalculateShot|SetAuxY 3e+01)
                  (goto _label))
                (:==
                  (Variables|CalculateShot|SetAuxY 75.0)
                  (goto _label))
                (:<
                  (Variables|CalculateShot|SetAuxY 125.0)
                  (goto _label))))))))))

(fn ConstructionScript)

(fn OnRepMaterial
  (Rendering|Material|CreateDynamicMaterialInstance (Variables|Default|GetSphere) 0 (Variables|Default|GetMaterial) "None" :!class /Script/Engine.PrimitiveComponent))

(fn OnRepImpulse
  (bind _sphere (Variables|Default|GetSphere))
  (bind _impulse (Variables|CalculateShot|GetImpulse))
  (Class|PrimitiveComponent|SetAllPhysicsLinearVelocity _sphere "0,-100.000000, 0" false)
  (Physics|AddImpulse _sphere (Math|Vector|MakeVector 0.0 (.y _impulse) (.z _impulse)) "None" true))

(fn OnRepIsParticleAnim
  (bind _trail (Variables|Default|GetTrail))
  (if (not (Variables|Default|GetIsParticleAnim))
    (Effects|Particles|Trails|EndTrails _trail)
    (else
      (Effects|Particles|Trails|BeginTrails _trail "trail1" "trail2" "ETrailWidthMode_FromFirst" 1.0))))

(fn OnRepCurrentMaterial
  (Rendering|Material|SetMaterial (Variables|Default|GetSphere) 0 (Variables|Materials|GetCurrentMaterial)))

(fn OnRepPlayerName
  (Rendering|Components|TextRender|SetText (Variables|Default|GettxtPlayer) (Variables|Default|GetPlayerName)))